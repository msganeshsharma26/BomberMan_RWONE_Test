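; Bomb for TD_PLayer1 that detonates one second after it begins play, then destroys itself.
; For each TD_PLayer1 actor found in the level, it decrements that actor's BombAmount1 and calls Explode.
; Explode spawns four Bomb_explosion_1 actors at the Sphere component's location, rotated along positive and negative X and Y to form a cross.
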(event Custom|Explode
  (for _array_element (Utilities|Array|MakeArray "1.000000, 0, 0" "0,1.000000, 0" "-1.000000, 0, 0" "0,-1.000000, 0")
    (Game|SpawnActorfromClass "/Game/Map/BluePrints/Bomb_explosion_1.Bomb_explosion_1_C" (Math|Transform|MakeTransform (Transformation|GetWorldLocation (Variables|Default|GetSphere)) (Math|Conversions|RotationFromXVector _array_element) "1,1,1") "Undefined" 0 0)))

(event EventBeginPlay
  (Utilities|FlowControl|Delay 1.0)
  (bind _outactors (Actor|GetAllActorsOfClass "/Game/LocalMultiplayer/TD_PLayer1.TD_PLayer1_C"))
  (for _array_element _outactors
    (Math|Integer|DecrementInt (Variables|/Game/LocalMultiplayer/TD_PLayer1.TD_PLayer1_C|GetBombAmount_1 _array_element)
      (:%20%20
        (CallFunction|Explode))))
  (Actor|DestroyActor))

(fn ConstructionScript)
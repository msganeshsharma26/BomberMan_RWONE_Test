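; Bomb explosion actor that travels forward as a blast, destroying players and breakable walls it overlaps.
; BeginPlay caches the game instance and box-traces for static obstacles, storing the hit distance in Length, which this graph never reads.
; Tick sweeps the actor forward until it covers Player1's explosion length, then stops and destroys itself after a delay.
; While moving, its box overlap kills TD_PLayer1 and triggers wall drop chances before destroying walls.
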(event OnComponentBeginOverlap(Box)
  (params (OverlappedComponent :type Primitive%20Component%20Object%20Reference) (OtherActor :type Actor%20Object%20Reference) (OtherComp :type Primitive%20Component%20Object%20Reference) (OtherBodyIndex :type Integer) (bFromSweep :type Boolean) (SweepResult :type Hit%20Result%20Structure%20%28by%20ref%29))
  (bind _stop_ (Variables|Default|Getstop?))
  (Utilities|FlowControl|Sequence
    (:then_0
      (if (not _stop_)
        (bind _astd_player_1 (Utilities|Casting|CastToTD_PLayer1 OtherActor))
        (Actor|DestroyActor _astd_player_1)))
    (:then_1
      (if (not _stop_)
        (bind _asbreakable_wall (Utilities|Casting|CastToBreakableWall OtherActor))
        (Default|DropChance _asbreakable_wall)
        (Actor|DestroyActor OtherActor)))))

(event EventBeginPlay
  (Utilities|FlowControl|Sequence
    (:then_0
      (bind _asnew_game_instance (Utilities|Casting|CastToNewGameInstance (Game|GetGameInstance)))
      (Variables|Default|SetGameInstance _asnew_game_instance))
    (:then_1
      (Variables|Default|SetstartLocation (Transformation|GetActorLocation))
      (bind (_outhit _returnvalue) (Class|KismetSystemLibrary|BoxTraceSingleforObjects (Variables|Default|GetstartLocation) (+ (* (Transformation|GetActorForwardVector) (Variables|/Game/Blueprints/NewGameInstance.NewGameInstance_C|GetPlayer1EplosionLength (Variables|Default|GetGameInstance))) (Variables|Default|GetstartLocation)) "20.000000,20.000000,20.000000" "0, 0, 0" (Utilities|Array|MakeArray "ObjectTypeQuery1") false 0 "ForDuration" true))
      (if _returnvalue
        (Variables|Default|Setlength (.Distance (Collision|BreakHitResult _outhit)))))))

(event EventTick
  (params (DeltaSeconds :type Float%20%28single-precision%29))
  (if (not (Variables|Default|Getstop?))
    (Transformation|AddActorWorldOffset (* (Transformation|GetActorForwardVector) (* (Variables|Default|Getspeed) DeltaSeconds)) true)
    (if (>= (Math|Vector|VectorLength (- (Variables|Default|GetstartLocation) (Transformation|GetActorLocation))) (Variables|/Game/Blueprints/NewGameInstance.NewGameInstance_C|GetPlayer1EplosionLength (Variables|Default|GetGameInstance)))
      (Variables|Default|Setstop? true)
      (Utilities|FlowControl|Delay 0.5)
      (Actor|DestroyActor))))

(fn ConstructionScript)
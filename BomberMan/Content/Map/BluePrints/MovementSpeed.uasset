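; MovementSpeed is a pickup Blueprint that boosts a player's force value when touched.
; Its Box overlap accepts only actors whose class is exactly TD_PLayer1, then casts to it.
; PlayerIndexCache selects whether Player1ForceValue or Player2ForceValue gets a fixed increase, and the pickup then destroys itself.
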(event OnComponentBeginOverlap(Box)
  (params (OverlappedComponent :type Primitive%20Component%20Object%20Reference) (OtherActor :type Actor%20Object%20Reference) (OtherComp :type Primitive%20Component%20Object%20Reference) (OtherBodyIndex :type Integer) (bFromSweep :type Boolean) (SweepResult :type Hit%20Result%20Structure%20%28by%20ref%29))
  (if (== (Utilities|GetClass OtherActor) "/Game/LocalMultiplayer/TD_PLayer1.TD_PLayer1_C")
    (bind _astd_player_1 (Utilities|Casting|CastToTD_PLayer1 OtherActor))
    (if (== (Variables|/Game/LocalMultiplayer/TD_PLayer1.TD_PLayer1_C|GetPlayerIndexCache _astd_player_1) 0)
      (Variables|/Game/LocalMultiplayer/TD_PLayer1.TD_PLayer1_C|SetPlayer1ForceValue _astd_player_1 (+ (Variables|/Game/LocalMultiplayer/TD_PLayer1.TD_PLayer1_C|GetPlayer1ForceValue _astd_player_1) 5e+02))
      (else
        (Variables|/Game/LocalMultiplayer/TD_PLayer1.TD_PLayer1_C|SetPlayer2ForceValue _astd_player_1 (+ (Variables|/Game/LocalMultiplayer/TD_PLayer1.TD_PLayer1_C|GetPlayer2ForceValue _astd_player_1) 5e+02))))
    (Actor|DestroyActor)))

(fn ConstructionScript)
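; Breakable map wall that can drop a power-up pickup at its Cube's location through DropChance.
; DropChance runs cascading random checks, spawning at most one of a bomb amount booster, explosion length or movement speed pickup.
; Each comparison makes its own roll, including both bounds of the speed check, so later odds are conditional rather than slices of one roll.
; The file shows no breaking logic or caller for DropChance.
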(fn ConstructionScript)

(fn DropChance
  (bind _returnvalue (Math|Random|RandomFloatinRange 0.0 1e+02))
  (bind _cube (Variables|Default|GetCube))
  (bind _returnvalue_2 (Transformation|GetWorldLocation _cube))
  (bind _returnvalue_3 (Math|Conversions|ToTransform(Vector) _returnvalue_2))
  (if (< _returnvalue 15.0)
    (Game|SpawnActorfromClass "/Game/Map/BluePrints/BombAmountBooster.BombAmountBooster_C" _returnvalue_3 "Undefined" 0 0)
    (elif (> _returnvalue 85.0)
      (Game|SpawnActorfromClass "/Game/Map/BluePrints/Explosion_Length.Explosion_Length_C" _returnvalue_3 "Undefined" 0 0)
      (elif (and (< _returnvalue 7e+01) (> _returnvalue 4e+01))
        (Game|SpawnActorfromClass "/Game/Map/BluePrints/MovementSpeed.MovementSpeed_C" _returnvalue_3 "Undefined" 0 0)))))
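; Bomb explosion blast for player 1 that travels along its forward vector, destroying TD_PLayer1 characters and BreakableWalls it overlaps.
; On BeginPlay it takes its range from the player's Player1Explosion, then shortens it with a box trace against WorldStatic objects.
; Tick moves it with sweep until it covers that range, then stops dealing damage and destroys itself after a short delay.
; Destroyed walls first roll DropChance.
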(event OnComponentBeginOverlap(Box)
  (params (OverlappedComponent :type Primitive%20Component%20Object%20Reference) (OtherActor :type Actor%20Object%20Reference) (OtherComp :type Primitive%20Component%20Object%20Reference) (OtherBodyIndex :type Integer) (bFromSweep :type Boolean) (SweepResult :type Hit%20Result%20Structure%20%28by%20ref%29))
  (bind _stop_ (Variables|Default|Getstop?))
  (Utilities|FlowControl|Sequence
    (:then_0
      (if (not _stop_)
        (bind _astd_player_1 (Utilities|Casting|CastToTD_PLayer1 OtherActor))
        (Actor|DestroyActor _astd_player_1)))
    (:then_1
      (if (not _stop_)
        (bind _asbreakable_wall (Utilities|Casting|CastToBreakableWall OtherActor))
        (Default|DropChance _asbreakable_wall)
        (Actor|DestroyActor OtherActor)))))

(event Custom|Length_Value
  (bind _astd_player_1 (Utilities|Casting|CastToTD_PLayer1 (Game|GetPlayerCharacter 0)))
  (Variables|Default|Setlength (Variables|/Game/LocalMultiplayer/TD_PLayer1.TD_PLayer1_C|GetPlayer_1_Explosion _astd_player_1)))

(event EventBeginPlay
  (CallFunction|LengthValue)
  (Variables|Default|SetstartLocation (Transformation|GetActorLocation))
  (bind (_outhit _returnvalue) (Class|KismetSystemLibrary|BoxTraceSingleforObjects (Variables|Default|GetstartLocation) (+ (* (Transformation|GetActorForwardVector) (Variables|Default|Getlength)) (Variables|Default|GetstartLocation)) "15.000000,15.000000,15.000000" "0, 0, 0" (Utilities|Array|MakeArray "ObjectTypeQuery1") false 0 "ForDuration" true))
  (if _returnvalue
    (bind _output_get (Variables|Default|Setlength (.Distance (Collision|BreakHitResult _outhit))))
    (Development|PrintString (Utilities|String|ToString(Float) _output_get))))

(event EventTick
  (params (DeltaSeconds :type Float%20%28single-precision%29))
  (if (not (Variables|Default|Getstop?))
    (Transformation|AddActorWorldOffset (* (Transformation|GetActorForwardVector) (* (Variables|Default|Getspeed) DeltaSeconds)) true)
    (if (>= (Math|Vector|VectorLength (- (Variables|Default|GetstartLocation) (Transformation|GetActorLocation))) (Variables|Default|Getlength))
      (Variables|Default|Setstop? true)
      (Utilities|FlowControl|Delay 0.5)
      (Actor|DestroyActor))))

(fn ConstructionScript)
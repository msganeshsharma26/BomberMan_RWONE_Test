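; Explosion_Length is a pickup actor that increases the explosion value of the player who touches it, likely extending blast length.
; Its Box overlap event accepts only actors whose class is exactly TD_PLayer1, then uses PlayerIndexCache to raise either Player1Explosion or Player2Explosion on that actor by a fixed step.
; It prints which player collected it and destroys itself.
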(event OnComponentBeginOverlap(Box)
  (params (OverlappedComponent :type Primitive%20Component%20Object%20Reference) (OtherActor :type Actor%20Object%20Reference) (OtherComp :type Primitive%20Component%20Object%20Reference) (OtherBodyIndex :type Integer) (bFromSweep :type Boolean) (SweepResult :type Hit%20Result%20Structure%20%28by%20ref%29))
  (if (== (Utilities|GetClass OtherActor) "/Game/Blueprints/TD_PLayer1.TD_PLayer1_C")
    (bind _astd_player_1 (Utilities|Casting|CastToTD_PLayer1 OtherActor))
    (if (== (Variables|/Game/Blueprints/TD_PLayer1.TD_PLayer1_C|GetPlayerIndexCache _astd_player_1) 0)
      (Variables|/Game/Blueprints/TD_PLayer1.TD_PLayer1_C|SetPlayer_1_Explosion _astd_player_1 (+ (Variables|/Game/Blueprints/TD_PLayer1.TD_PLayer1_C|GetPlayer_1_Explosion _astd_player_1) 5e+01))
      (Development|PrintString "player_1")
      (else
        (Variables|/Game/Blueprints/TD_PLayer1.TD_PLayer1_C|SetPlayer_2_Explosion _astd_player_1 (+ (Variables|/Game/Blueprints/TD_PLayer1.TD_PLayer1_C|GetPlayer_2_Explosion _astd_player_1) 5e+01))
        (Development|PrintString "Player_2")))
    (Actor|DestroyActor)))

(fn ConstructionScript)
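; Directional arm of a bomb explosion, sized by player two's explosion stat, that kills players and breaks walls.
; On BeginPlay a forward box trace shortens its length at the first WorldStatic hit.
; Tick sweeps the actor forward to that length, then destroys it after a delay.
; While moving, box overlaps trigger wall drop chances and destruction, or destroy players and show a win or draw screen.
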(event OnComponentBeginOverlap(Box)
  (params (OverlappedComponent :type Primitive%20Component%20Object%20Reference) (OtherActor :type Actor%20Object%20Reference) (OtherComp :type Primitive%20Component%20Object%20Reference) (OtherBodyIndex :type Integer) (bFromSweep :type Boolean) (SweepResult :type Hit%20Result%20Structure%20%28by%20ref%29))
  (bind _returnvalue (Game|GetPlayerController 0))
  (bind _returnvalue_2 (Game|GetPlayerController 0))
  (bind _returnvalue_3 (Game|GetPlayerController 0))
  (bind _returnvalue_4 (Game|GetPlayerController 0))
  (bind _stop_ (Variables|Default|Getstop?))
  ;[1 1 1] Logic for the death of player if it collides with the bounding box
  (Utilities|FlowControl|Sequence
    (:then_0
      (if (not _stop_)
        (bind _astd_player_1 (Utilities|Casting|CastToTD_PLayer1 OtherActor))
        (if (== (Variables|/Game/Blueprints/TD_PLayer1.TD_PLayer1_C|GetPlayerIndexCache _astd_player_1) 0)
          (Actor|DestroyActor _astd_player_1)
          (Variables|Default|SetPlayer_1_Val 0)
          (Utilities|FlowControl|Delay 1.0)
          (if (== (Variables|Default|GetPlayer_1_Val) (Variables|Default|GetPlayer_2_Val))
            (Development|PrintString "draw")
            (bind _returnvalue_5 (UserInterface|CreateWidget "/Game/UI/Draw.Draw_C" _returnvalue_2))
            (UserInterface|Viewport|AddtoViewport _returnvalue_5 0)
            (Input|SetInputModeUIOnly _returnvalue_2 _returnvalue_5 "DoNotLock")
            (Variables|/Script/Engine.PlayerController|SetbShowMouseCursor _returnvalue_2 true)
            (else
              (Development|PrintString "Player1Dead")
              (bind _returnvalue_6 (UserInterface|CreateWidget "/Game/UI/Player2Win.Player2Win_C" _returnvalue_3))
              (UserInterface|Viewport|AddtoViewport _returnvalue_6 0)
              (Input|SetInputModeUIOnly _returnvalue_3 _returnvalue_6 "DoNotLock")
              (Variables|/Script/Engine.PlayerController|SetbShowMouseCursor _returnvalue_3 true)))
          (else
            (Actor|DestroyActor _astd_player_1)
            (Variables|Default|SetPlayer_2_Val 0)
            (Utilities|FlowControl|Delay 1.0)
            (if (== (Variables|Default|GetPlayer_1_Val) (Variables|Default|GetPlayer_2_Val))
              (Development|PrintString "draw")
              (bind _returnvalue_7 (UserInterface|CreateWidget "/Game/UI/Draw.Draw_C" _returnvalue_4))
              (UserInterface|Viewport|AddtoViewport _returnvalue_7 0)
              (Input|SetInputModeUIOnly _returnvalue_4 _returnvalue_7 "DoNotLock")
              (Variables|/Script/Engine.PlayerController|SetbShowMouseCursor _returnvalue_4 true)
              (else
                (Development|PrintString "Player2Dead")
                (bind _returnvalue_8 (UserInterface|CreateWidget "/Game/UI/Player1Win.Player1Win_C" _returnvalue))
                (UserInterface|Viewport|AddtoViewport _returnvalue_8 0)
                (Input|SetInputModeUIOnly _returnvalue _returnvalue_8 "DoNotLock")
                (Variables|/Script/Engine.PlayerController|SetbShowMouseCursor _returnvalue true)))))))
    (:then_1
      (if (not _stop_)
        (bind _asbreakable_wall (Utilities|Casting|CastToBreakableWall OtherActor))
        (Default|DropChance _asbreakable_wall)
        (Actor|DestroyActor OtherActor)))))

(event Custom|Length_Value
  ;[1 1 1] retrieving the value of explosion length from Player blueprint
  (bind _astd_player_1 (Utilities|Casting|CastToTD_PLayer1 (Game|GetPlayerCharacter 1)))
  (Variables|Default|Setlength (Variables|/Game/Blueprints/TD_PLayer1.TD_PLayer1_C|GetPlayer_2_Explosion _astd_player_1)))

(event EventBeginPlay
  ;[1 1 1] Calculationa for the single directional of spawning explosion
  (CallFunction|LengthValue)
  (Variables|Default|SetstartLocation (Transformation|GetActorLocation))
  (bind (_outhit _returnvalue) (Class|KismetSystemLibrary|BoxTraceSingleforObjects (Variables|Default|GetstartLocation) (+ (* (Transformation|GetActorForwardVector) (Variables|Default|Getlength)) (Variables|Default|GetstartLocation)) "30.000000,30.000000,30.000000" "0, 0, 0" (Utilities|Array|MakeArray "ObjectTypeQuery1") false 0 "ForDuration" true))
  (if _returnvalue
    (Variables|Default|Setlength (.Distance (Collision|BreakHitResult _outhit)))))

(event EventTick
  (params (DeltaSeconds :type Float%20%28single-precision%29))
  ;[1 1 1] Animating the bounding box for particle effect with speed
  (if (not (Variables|Default|Getstop?))
    (Transformation|AddActorWorldOffset (* (Transformation|GetActorForwardVector) (* (Variables|Default|Getspeed) DeltaSeconds)) true)
    (if (>= (Math|Vector|VectorLength (- (Variables|Default|GetstartLocation) (Transformation|GetActorLocation))) (Variables|Default|Getlength))
      (Variables|Default|Setstop? true)
      (Utilities|FlowControl|Delay 0.5)
      (Actor|DestroyActor))))

(fn ConstructionScript)
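; Player1 is a player-controlled Blueprint built around a physics-driven Cube that moves and drops bombs.
; The MoveUp and MoveRight axes apply mass-independent force along the cube's forward and right vectors, scaled by ForceStrength.
; Pressing Fire spawns a Bomb_1 above the cube and increments BombAmount until it reaches MaxBombAmount.
; Nothing in this graph decrements the bomb count.
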(event Input|ActionEvents|InputActionFire
  (params (Key :type Key%20Structure))
  (bind _cube (Variables|Default|GetCube))
  (bind _returnvalue (Transformation|GetWorldLocation _cube))
  (bind (_x _y _z) (Math|Vector|BreakVector _returnvalue))
  ;[1 1 1] Bomb Input with Condition
  (:Pressed
    (if (!= (Variables|Default|GetBombAmount) (Variables|Default|GetMaxBombAmount))
      (Game|SpawnActorfromClass "/Game/Map/BluePrints/Bomb_1.Bomb_1_C" (Math|Conversions|ToTransform(Vector) (Math|Vector|MakeVector _x _y (+ _z 2.5e+02))) "Undefined" 0 0)
      (Math|Integer|IncrementInt (Variables|Default|GetBombAmount)))))

(event Input|AxisEvents|InputAxisMoveRight
  (params (AxisValue :type Float%20%28single-precision%29))
  (bind _cube (Variables|Default|GetCube))
  ;[1 1 1] Movement Base on force applied to cube using Inputs
  (Physics|AddForce _cube (* (Math|Vector|GetRightVector _cube) (* (Variables|Default|GetForceStrength) AxisValue)) "None" true))

(event Input|AxisEvents|InputAxisMoveUp
  (params (AxisValue :type Float%20%28single-precision%29))
  (bind _cube (Variables|Default|GetCube))
  ;[1 1 1] Movement Base on force applied to cube using Inputs
  (Physics|AddForce _cube (* (Math|Vector|GetForwardVector _cube) (* AxisValue (Variables|Default|GetForceStrength))) "None" true))

(fn ConstructionScript)
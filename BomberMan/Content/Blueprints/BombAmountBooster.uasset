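; BombAmountBooster is a pickup actor that raises a player's maximum bomb count.
; When its Box is overlapped by a TD_PLayer1, PlayerIndexCache selects whether MaxBombAmount1 (index 0) or MaxBombAmount2 (any other index) is incremented.
; It copies the result to the matching MaxBomb1 or MaxBomb2 in NewGameInstance, intended for the UI, then destroys itself.
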(event OnComponentBeginOverlap(Box)
  (params (OverlappedComponent :type Primitive%20Component%20Object%20Reference) (OtherActor :type Actor%20Object%20Reference) (OtherComp :type Primitive%20Component%20Object%20Reference) (OtherBodyIndex :type Integer) (bFromSweep :type Boolean) (SweepResult :type Hit%20Result%20Structure%20%28by%20ref%29))
  (bind _returnvalue (Game|GetGameInstance))
  ;[1 1 1] Adding the value to maxbomb amount to respective UI and Player MaxbombAmount value
  (if (== (Utilities|GetClass OtherActor) "/Game/Blueprints/TD_PLayer1.TD_PLayer1_C")
    (bind _astd_player_1 (Utilities|Casting|CastToTD_PLayer1 OtherActor))
    (if (== (Variables|/Game/Blueprints/TD_PLayer1.TD_PLayer1_C|GetPlayerIndexCache _astd_player_1) 0)
      (bind _result (Math|Integer|IncrementInt (Variables|/Game/Blueprints/TD_PLayer1.TD_PLayer1_C|GetMaxBombAmount_1 _astd_player_1))
        (:%20%20
          (bind _asnew_game_instance (Utilities|Casting|CastToNewGameInstance _returnvalue))
          (Variables|/Game/Blueprints/NewGameInstance.NewGameInstance_C|SetMaxBomb1 _asnew_game_instance _result)
          (Actor|DestroyActor)))
      (else
        (bind _result_2 (Math|Integer|IncrementInt (Variables|/Game/Blueprints/TD_PLayer1.TD_PLayer1_C|GetMaxBombAmount_2 _astd_player_1))
          (:%20%20
            (bind _asnew_game_instance_2 (Utilities|Casting|CastToNewGameInstance _returnvalue))
            (Variables|/Game/Blueprints/NewGameInstance.NewGameInstance_C|SetMaxBomb2 _asnew_game_instance_2 _result_2)
            (Actor|DestroyActor)))))))

(fn ConstructionScript)
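; Player 1's timed bomb actor, which explodes in four directions after a short fixed delay.
; When the delay from BeginPlay ends, it decrements BombAmount1 on every TD_PLayer1 actor, calls Explode inside that same loop, then destroys itself.
; Explode spawns four Bomb_explosion_1 actors at the sphere's location, rotated along the positive and negative X and Y axes.
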(event Custom|Explode
  ;[1 1 1] Four way directional explosion spawning logic
  (for _array_element (Utilities|Array|MakeArray "1.000000, 0, 0" "0,1.000000, 0" "-1.000000, 0, 0" "0,-1.000000, 0")
    (Game|SpawnActorfromClass "/Game/Blueprints/Bomb_explosion_1.Bomb_explosion_1_C" (Math|Transform|MakeTransform (Transformation|GetWorldLocation (Variables|Default|GetSphere)) (Math|Conversions|RotationFromXVector _array_element) "1,1,1") "Undefined" 0 0)))

(event EventBeginPlay
  ;[1 1 1] Destroy bomb after instantiating
  (Utilities|FlowControl|Delay 3.0)
  (bind _outactors (Actor|GetAllActorsOfClass "/Game/Blueprints/TD_PLayer1.TD_PLayer1_C"))
  (for _array_element _outactors
    (Math|Integer|DecrementInt (Variables|/Game/Blueprints/TD_PLayer1.TD_PLayer1_C|GetBombAmount_1 _array_element)
      (:%20%20
        (CallFunction|Explode))))
  (Actor|DestroyActor))

(fn ConstructionScript)
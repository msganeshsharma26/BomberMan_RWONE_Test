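; Top-down player character for a two-player bomb game, moved along world axes by input.
; Space and the gamepad bottom button spawn separate bomb classes above the mesh, each with its own count limit.
; Tick uses the cached player index to set the second player's material and apply that player's pickup-driven force as max acceleration.
; RotateToFace yaws the first controller toward the cursor hit, but nothing here calls it.
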(event EventTick
  (params (DeltaSeconds :type Float%20%28single-precision%29))
  (bind _charactermovement (Variables|Character|GetCharacterMovement))
  (Utilities|FlowControl|Sequence
    (:then_0
      ;[1 1 1] Set Material for 2nd Player
      (if (== (Variables|Default|GetPlayerIndexCache) 1)
        (Rendering|Material|SetMaterial (Variables|Character|GetMesh) 0 "/Game/Textures/TD_Player1_Mat.TD_Player1_Mat")))
    (:then_1
      ;[1 1 1] Speed value got from the pickups, applying to the respective variables
      (if (== (Variables|Default|GetPlayerIndexCache) 1)
        (bind _output_get (Variables|Default|SetForceStrength (Variables|Default|GetPlayer2ForceValue)))
        (Variables|/Script/Engine.CharacterMovementComponent|SetMaxAcceleration _charactermovement _output_get)
        (else
          (bind _output_get_2 (Variables|Default|SetForceStrength (Variables|Default|GetPlayer1ForceValue)))
          (Variables|/Script/Engine.CharacterMovementComponent|SetMaxAcceleration _charactermovement _output_get_2))))))

(event Input|AxisEvents|InputAxisMoveUp
  (params (AxisValue :type Float%20%28single-precision%29))
  ;[1 1 1] Movement Inputs
  (Pawn|Input|AddMovementInput "90.000000, 0, 0" AxisValue false))

(event Input|AxisEvents|InputAxisMoveRight
  (params (AxisValue :type Float%20%28single-precision%29))
  ;[1 1 1] Movement Inputs
  (Pawn|Input|AddMovementInput "0,90.000000, 0" AxisValue false))

(event Input|KeyboardEvents|SpaceBar
  (params (Key :type Key%20Structure :default "None"))
  (bind _mesh (Variables|Character|GetMesh))
  (bind _returnvalue (Transformation|GetWorldLocation _mesh))
  (bind (_x _y _z) (Math|Vector|BreakVector _returnvalue))
  ;[1 1 1] Spawning Bombs
  (:Pressed
    (if (!= (Variables|Default|GetBombAmount_1) (Variables|Default|GetMaxBombAmount_1))
      (Game|SpawnActorfromClass "/Game/Blueprints/Bomb_1.Bomb_1_C" (Math|Conversions|ToTransform(Vector) (Math|Vector|MakeVector _x _y (+ _z 2.5e+02))) "Undefined" 0 0)
      (Math|Integer|IncrementInt (Variables|Default|GetBombAmount_1)))))

(event Input|GamepadEvents|GamepadFaceButtonBottom
  (params (Key :type Key%20Structure :default "None"))
  (bind _mesh (Variables|Character|GetMesh))
  (bind _returnvalue (Transformation|GetWorldLocation _mesh))
  (bind (_x _y _z) (Math|Vector|BreakVector _returnvalue))
  ;[1 1 1] Spawning Bombs
  (:Pressed
    (if (!= (Variables|Default|GetBombAmount_2) (Variables|Default|GetMaxBombAmount_2))
      (Game|SpawnActorfromClass "/Game/Blueprints/Bomb_2.Bomb_2_C" (Math|Conversions|ToTransform(Vector) (Math|Vector|MakeVector _x _y (+ _z 2.5e+02))) "Undefined" 0 0)
      (Math|Integer|IncrementInt (Variables|Default|GetBombAmount_2)))))

(fn ConstructionScript)

(fn RotatetoFace
  (bind _returnvalue (Game|GetPlayerController 0))
  ;[1 1 1] Function for rotation of the Player accoding to the input direction
  (Pawn|SetControlRotation _returnvalue (Math|Rotator|MakeRotator 0.0 0.0 (.yaw (Math|Rotator|FindLookatRotation (Transformation|GetActorLocation self) (.Location (Collision|BreakHitResult (.HitResult (Game|Player|GetHitResultUnderCursorbyChannel _returnvalue "TraceTypeQuery1" true)))))))))